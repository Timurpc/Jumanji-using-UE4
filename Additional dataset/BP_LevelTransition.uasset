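; Level transition trigger that opens a named level when a player character holding the required key type overlaps it.
; On overlap it casts to ThirdPersonCharacter and scans OwnedKeys, removing a matching key.
; It copies the remaining keys to PlayerKeys on TestGameInstance so they carry across the level load, then opens LevelName.
; The loop has no break after a match.
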(event `self.Overlap.OnComponentBeginOverlap`
  (params (OverlappedComponent :type "PrimitiveComponent Object Reference") (OtherActor :type "Actor Object Reference") (OtherComp :type "PrimitiveComponent Object Reference") (OtherBodyIndex :type Integer) (bFromSweep :type Boolean) (SweepResult :type "HitResult Structure (by ref)"))
  (bind _asthird_person_character (cast `/Game/ThirdPersonBP/Blueprints/ThirdPersonCharacter` OtherActor))
  (bind _ownedkeys (`/Game/ThirdPersonBP/Blueprints/ThirdPersonCharacter.OwnedKeys` _asthird_person_character))
  (for (_array_element _array_index) _ownedkeys
    (if (`|EnumEquality` _array_element (`self.RequiredKeyType`))
      (`KismetArrayLibrary.Array_Remove` _ownedkeys _array_index)
      (bind _astest_game_instance (cast `/Game/TestGameInstance` (`GameplayStatics.GetGameInstance`)))
      (set `/Game/TestGameInstance.PlayerKeys` _ownedkeys _astest_game_instance)
      (`GameplayStatics.OpenLevel` (`self.LevelName`)))))

(fn `UserConstructionScript`)